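; Enemy AI that roams random reachable points, chases pawns seen through PawnSensing, and resumes roaming after a retriggerable delay without a sighting.
; On BeginPlay, its max health scales with the first found player character's level.
; Damage passes through server/multicast-named events, reducing a fixed overall pool and applying the same fractional loss to the scaled CurrentHealth.
; A looping timer and CurrentHealth OnRep refresh the health bar widget.
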(event OnSeePawn(PawnSensing)
  (params (Pawn :type Pawn%20Object%20Reference))
  (Utilities|FlowControl|Sequence
    (:then_0
      (AI|AIMoveTo self "0, 0, 0" Pawn 5.0 false))
    (:then_1
      (Utilities|FlowControl|RetriggerableDelay 2.5)
      (CallFunction|RandomRoaming))))

(event Custom|SRV_Damge
  (params (Damage :type Float%20%28double-precision%29))
  (Variables|Default|SetOriginalOverallHealth (Variables|Default|GetOverallHealth))
  (bind _output_get (Variables|Default|SetHealthPercentageLost (/ Damage (Variables|Default|GetOriginalOverallHealth))))
  (Development|PrintString (Utilities|String|ToString(Float) _output_get))
  (bind _output_get_2 (Variables|Default|SetOverallHealth (Math|Float|Clamp(Float) (- (Variables|Default|GetOverallHealth) Damage) 0.0 1e+03)))
  (Development|PrintString (Utilities|String|ToString(Float) _output_get_2))
  (CallFunction|MCHealthUpdate))

(event Custom|UpdateHealthText
  (bind _aswb_enemy_health_bar (Utilities|Casting|CastToWB_EnemyHealthBar (UserInterface|GetWidget (Variables|Default|GetHealthBarWidget))))
  (Rendering|Components|TextRender|SetText (Variables|/Game/Blueprints/Enemy/WB_EnemyHealthBar.WB_EnemyHealthBar_C|GetTXT_Health _aswb_enemy_health_bar) (Utilities|Text|FormatText "{CurrentHealth} / {BaseMaxHealth}" (Math|Float|Truncate (Variables|Default|GetCurrentHealth)) (Math|Float|Truncate (Variables|Default|GetMaxHealth))))
  (Variables|Default|SetCurrentHealth (Math|Float|Clamp(Float) (- (Variables|Default|GetCurrentHealth) (* (Variables|Default|GetHealthPercentageLost) (Variables|Default|GetCurrentHealth))) 0.0 (Variables|Default|GetMaxHealth))))

(event Custom|RandomRoaming
  (AI|AIMoveTo self (.RandomLocation (AI|Navigation|GetRandomReachablePointinRadius (Transformation|GetActorLocation) 1e+03 0 0)) 0 5.0 false
    (:OnSuccess
      (CallFunction|RandomRoaming))))

(event Custom|SetUpHealthBar
  (bind _aswb_enemy_health_bar (Utilities|Casting|CastToWB_EnemyHealthBar (UserInterface|GetWidget (Variables|Default|GetHealthBarWidget))))
  (Progress|SetPercent (Variables|/Game/Blueprints/Enemy/WB_EnemyHealthBar.WB_EnemyHealthBar_C|GetEnemyHealthBar _aswb_enemy_health_bar) (/ (Variables|Default|GetCurrentHealth) (Variables|Default|GetMaxHealth)))
  (Rendering|Components|TextRender|SetText (Variables|/Game/Blueprints/Enemy/WB_EnemyHealthBar.WB_EnemyHealthBar_C|GetTXT_Health _aswb_enemy_health_bar) (Utilities|Text|FormatText "{CurrentHealth} / {BaseMaxHealth}" (Math|Float|Truncate (Variables|Default|GetCurrentHealth)) (Math|Float|Truncate (Variables|Default|GetMaxHealth)))))

(event Custom|MC_HealthUpdate
  (Utilities|Time|SetTimerbyFunctionName 0 "SetUpHealthBar" 0.1 true)
  (CallFunction|UpdateHealthText))

(event Custom|CL_PlayerLevelHealths
  (CallFunction|FGetPlayerLevel))

(event Custom|Damage
  (params (Damage :type Float%20%28double-precision%29))
  (CallFunction|SRVDamge Damage))

(event EventBeginPlay
  (Utilities|FlowControl|Delay 0.1)
  (CallFunction|CLPlayerLevelHealths)
  (CallFunction|MCHealthUpdate)
  (Variables|Default|SetOverallHealth 1e+03)
  (CallFunction|RandomRoaming))

(event Game|Damage|EventAnyDamage
  (params (Damage :type Float%20%28single-precision%29) (DamageType :type Damage%20Type%20Object%20Reference) (InstigatedBy :type Controller%20Object%20Reference) (DamageCauser :type Actor%20Object%20Reference))
  (CallFunction|Damage Damage))

(fn ConstructionScript)

(fn FGetPlayerLevel
  (Utilities|Casting|CastToPlayer_Charcter_Base (Game|GetPlayerCharacter 0))
  (bind _outactors (Actor|GetAllActorsOfClass "/Game/Blueprints/Player/Player_Charcter_Base.Player_Charcter_Base_C"))
  (Development|PrintString (Utilities|String|ToString(Integer) (Variables|/Game/Blueprints/Player/Player_Charcter_Base.Player_Charcter_Base_C|GetPlayerLevel (Utilities|Array|Get(acopy) _outactors))))
  (bind _output_get (Variables|Default|SetMaxHealth (Math|Conversions|ToFloat(Integer) (* (Variables|/Game/Blueprints/Player/Player_Charcter_Base.Player_Charcter_Base_C|GetPlayerLevel (Utilities|Array|Get(acopy) _outactors)) 100))))
  (Variables|Default|SetCurrentHealth _output_get)
  (Development|PrintString (Utilities|String|ToString(Float) (Variables|Default|GetMaxHealth))))

(fn GetPlayerBaseRef
  (return 0))

(fn OnRepCurrentHealth
  (bind _aswb_enemy_health_bar (Utilities|Casting|CastToWB_EnemyHealthBar (UserInterface|GetWidget (Variables|Default|GetHealthBarWidget))))
  (Rendering|Components|TextRender|SetText (Variables|/Game/Blueprints/Enemy/WB_EnemyHealthBar.WB_EnemyHealthBar_C|GetTXT_Health _aswb_enemy_health_bar) (Utilities|Text|FormatText "{CurrentHealth} / {BaseMaxHealth}" (Math|Float|Truncate (Variables|Default|GetCurrentHealth)) (Math|Float|Truncate (Variables|Default|GetMaxHealth)))))