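; BP_EnemySpawner is an actor that spawns a wave of BP_EnemyAI enemies around itself.
; After a 30-second delay following BeginPlay, it starts a looping timer that calls SRV_SpawnEnemy.
; Each tick spawns an enemy at a random reachable navmesh point within a radius of the spawner.
; It increments the spawn count on IP_GameMode and clears the timer once MaxEnemies is reached.
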(event Custom|SRV_SpawnEnemy
  (bind _ip_game_mode (Variables|Default|GetIP%20Game%20Mode))
  (Game|SpawnActorfromClass "/Game/Blueprints/Enemy/BP_EnemyAI.BP_EnemyAI_C" (Math|Transform|MakeTransform (.RandomLocation (AI|Navigation|GetRandomReachablePointinRadius (Transformation|GetActorLocation) 5e+03 0 0)) "0, 0, 0" "1.000000,1.000000,1.000000") "Undefined" "MultiplyWithRoot" 0 0)
  (bind _result (Math|Integer|IncrementInt (Variables|/Game/Blueprints/Player/IP_GameMode.IP_GameMode_C|GetNumberOfEnemiesSpawned _ip_game_mode))
    (:%20%20
      (if (>= _result (Variables|/Game/Blueprints/Player/IP_GameMode.IP_GameMode_C|GetMaxEnemies _ip_game_mode))
        (Utilities|Time|ClearandInvalidateTimerbyHandle (Variables|Default|GetSpawnEnemyTimer))))))

(event Custom|StartWave
  (bind _returnvalue (Utilities|Time|SetTimerbyEvent (delegate Custom|SRV_SpawnEnemy) 5.0 true))
  (Variables|Default|SetSpawnEnemyTimer _returnvalue))

(event EventBeginPlay
  (bind _asip_game_mode (Utilities|Casting|CastToIP_GameMode (Game|GetGameMode)))
  (Variables|Default|SetIP%20Game%20Mode _asip_game_mode)
  (Utilities|FlowControl|Delay 3e+01)
  (CallFunction|StartWave))

(fn ConstructionScript)