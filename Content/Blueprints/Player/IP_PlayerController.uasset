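; Player controller that owns the game's UI, switching between main menu and in-game HUD based on whether the current level is Main_Menu.
; The menu level hides the player mesh and uses UI-only input, while other levels show crosshair and main HUD with game-only input.
; ShowHideWidget requests route to functions that lazily create or remove widgets by enum; showing Menus also creates server creation and browser widgets.
; PauseMenu adds a pause widget with cursor and UI-only input.
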(event Custom|ShowHideWidget
  (params (Widget :type Game_UI%20Enum :default "NewEnumerator0") (Show :type Boolean))
  (CallFunction|CLShowHideWidget Widget Show))

(event Custom|CL_ShowHideWidget
  (params (Widget :type Game_UI%20Enum :default "NewEnumerator0") (Show :type Boolean))
  (if Show
    (CallFunction|FShowWidget Widget)
    (else
      (CallFunction|FHideWidget Widget))))

(event Custom|PauseMenu
  (bind _returnvalue (Game|GetPlayerController 0))
  (bind _returnvalue_2 (UserInterface|CreateWidget "/Game/UI/WB_PauseMenu.WB_PauseMenu_C"))
  (bind _output_get (Variables|Default|SetPauseMenuVar _returnvalue_2))
  (UserInterface|Viewport|AddtoViewport _output_get 0)
  (Input|SetInputModeUIOnly _returnvalue 0 "DoNotLock" false)
  (Variables|/Script/Engine.PlayerController|SetbShowMouseCursor _returnvalue true))

(event EventBeginPlay
  (bind _returnvalue (Game|GetPlayerController 0))
  (bind _returnvalue_2 (Game|GetCurrentLevelName true))
  (if (Utilities|Enum|Equal(Enum) _returnvalue_2 "Main_Menu")
    (CallFunction|ShowHideWidget "NewEnumerator2" true)
    (bind _asplayer_charcter_base (Utilities|Casting|CastToPlayer_Charcter_Base (Game|GetPlayerCharacter 0)))
    (Rendering|SetVisibility (Variables|/Script/Engine.Character|GetMesh _asplayer_charcter_base) false false)
    (Input|SetInputModeUIOnly (Game|GetPlayerController 0) 0 "DoNotLock" false)
    (else
      (CallFunction|ShowHideWidget "NewEnumerator0" true)
      (CallFunction|ShowHideWidget "NewEnumerator1" true)
      (CallFunction|ShowHideWidget "NewEnumerator2" false)
      (Input|SetInputModeGameOnly _returnvalue false)
      (Variables|/Script/Engine.PlayerController|SetbShowMouseCursor _returnvalue false))))

(fn ConstructionScript)

(fn FShowWidget
  (params (Widget :type Game_UI%20Enum :default "NewEnumerator0"))
  (switch Utilities|FlowControl|Switch|SwitchonGame_UI Widget
    (:NewEnumerator1
      (Variables|Default|GetWB_Main
        (:then
          _)
        (:else
          (bind _returnvalue (UserInterface|CreateWidget "/Game/UI/WB_Main.WB_Main_C"))
          (bind _output_get (Variables|Default|SetWB_Main _returnvalue))))
      (UserInterface|Viewport|AddtoViewport _output_get 0))
    (:NewEnumerator0
      (Variables|Default|GetCrosshair
        (:then
          _)
        (:else
          (bind _returnvalue_2 (UserInterface|CreateWidget "/Game/UI/WB_Crosshair.WB_Crosshair_C"))
          (bind _output_get_2 (Variables|Default|SetCrosshair _returnvalue_2))))
      (UserInterface|Viewport|AddtoViewport _output_get_2 0))
    (:NewEnumerator2
      (Variables|Default|GetMainMenu
        (:then
          _)
        (:else
          (bind _returnvalue_3 (UserInterface|CreateWidget "/Game/UI/WB_MainMenu.WB_MainMenu_C"))
          (bind _output_get_3 (Variables|Default|SetMainMenu _returnvalue_3))))
      (UserInterface|Viewport|AddtoViewport _output_get_3 0)
      (bind _returnvalue_4 (UserInterface|CreateWidget "/Game/UI/WB_CreateServer.WB_CreateServer_C"))
      (Variables|Default|SetCreateServer _returnvalue_4)
      (bind _returnvalue_5 (UserInterface|CreateWidget "/Game/UI/WB_ServerBrowser.WB_ServerBrowser_C"))
      (Variables|Default|SetServerBrowser _returnvalue_5))))

(fn FHideWidget
  (params (Widget :type Game_UI%20Enum :default "NewEnumerator0"))
  (switch Utilities|FlowControl|Switch|SwitchonGame_UI Widget
    (:NewEnumerator1
      (bind _wb_main (Variables|Default|GetWB_Main)
        (:then
          (Widget|RemovefromParent _wb_main))
        (:else)))
    (:NewEnumerator0
      (bind _crosshair (Variables|Default|GetCrosshair)
        (:then
          (Widget|RemovefromParent _crosshair))
        (:else)))
    (:NewEnumerator2
      (bind _mainmenu (Variables|Default|GetMainMenu)
        (:then
          (Widget|RemovefromParent _mainmenu))
        (:else)))))

(fn GetPlayerControllerRef
  (return self))