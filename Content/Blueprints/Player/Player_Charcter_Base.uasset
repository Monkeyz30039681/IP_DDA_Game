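; Base multiplayer player character with Enhanced Input movement, pistol and rifle pickup and switching, hitscan shooting, reloading and regenerating health.
; Inputs call server events, which multicast montages and sound and push ammo and health to the owning client's HUD.
; RepNotifies attach weapons to hand or holster sockets; timers drive automatic fire and regeneration.
; A random player level scales damage against "Enemy"-tagged actors; the zero-health Death check is unconnected.
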(event Custom|SRV_Crouch
  (params (bCrouch :type Boolean))
  ;[1 1 1] Player Movment
  (CallFunction|FCrouch bCrouch))

(event Custom|SRV_Walk
  (params (bWalk :type Boolean))
  ;[1 1 1] Player Movment
  (CallFunction|FWalk bWalk))

(event Custom|CanPickUpAgain
  ;[1 1 1] Equip and Switch
  (Utilities|FlowControl|DoOnce false) ; enters at Reset
)

(event Custom|SRV_SwitchWeapon
  (params (WeaponTypeToFind :type Weapon_Type%20Enum :default "NewEnumerator0"))
  ;[1 1 1] Equip and Switch
  (bind (_weaponfound _weapon) (Utilities|MWeaponTypeInventChecker WeaponTypeToFind :!label _label)
    (:LoopBody
      (if _weaponfound
        (Variables|Default|SetbWeaponFoundInInvent true)
        (goto _label Break%20Loop)))
    (:LoopCompleted
      (if (Variables|Default|GetbWeaponFoundInInvent)
        (if (Utilities|Enum|Equal(Enum) (Variables|Default|GetEquippedWeapon) "NewEnumerator0")
          (bind _output_get (Variables|Default|SetEquipWeapon _weapon :!label _label_2))
          (Variables|Default|SetEquipedWeapon _output_get)
          (CallFunction|SetEquipedWeapon WeaponTypeToFind)
          (CallFunction|SetIsEquippingWeapon true)
          (Utilities|FlowControl|Delay 0.05)
          (CallFunction|CLUpdateAmmoUI (Variables|/Game/Blueprints/Weapons/Weapon_Base.Weapon_Base_C|GetCurrentAmmo (Variables|Default|GetEquipedWeapon)) (Variables|/Game/Blueprints/Weapons/Weapon_Base.Weapon_Base_C|GetCurrentReserveAmmo (Variables|Default|GetEquipedWeapon)))
          (CallFunction|CLDisplayAmmoUI true)
          (Variables|Default|SetUnequipWeapon 0)
          (Variables|Default|SetEquipWeapon 0)
          (Variables|Default|SetbWeaponFoundInInvent false)
          (else
            (bind (_weaponfound_2 _weapon_2) (Utilities|MWeaponTypeInventChecker (Variables|Default|GetEquippedWeapon) :!label _label_3)
              (:LoopBody
                (if _weaponfound_2
                  (Variables|Default|SetUnequipWeapon _weapon_2)
                  (goto _label_3 Break%20Loop)))
              (:LoopCompleted
                (goto _label_2)))))))))

(event Custom|SRV_ShootingWeapon
  (params (Weapon :type Weapon%20Base%20Object%20Reference) (bShootWeapon :type Boolean) (BulletStart :type Vector) (BulletEnd :type Vector))
  ;[1 1 1] Shooting, realoding, ammo
  (Utilities|IsValid Weapon
    (:Is%20Valid
      (if bShootWeapon
        (Utilities|FlowControl|DoOnce false
          (:Completed
            (CallFunction|FirstShot)
            (bind _returnvalue (Utilities|Time|SetTimerbyEvent (delegate Custom|ShootWeaponLoop) (.FireRate (Utilities|Struct|BreakWeapon_Info (CallFunction|FGetWeaponInfo (Variables|/Game/Blueprints/Weapons/Weapon_Base.Weapon_Base_C|GetWeaponName Weapon)))) true))
            (Variables|Default|SetShootWeaponHandle _returnvalue)))
        (elif (Utilities|Time|IsValidTimerHandle (Variables|Default|GetShootWeaponHandle))
          (Utilities|Time|ClearandInvalidateTimerbyHandle (Variables|Default|GetShootWeaponHandle))
          (CallFunction|CanShootAgain))))))

(event Custom|MC_SwitchWeapon
  (params (MontageToPlay :type Anim%20Montage%20Object%20Reference))
  ;[1 1 1] Shooting, realoding, ammo
  (Animation|Montage|PlayMontage (Variables|Character|GetMesh) MontageToPlay
    (:OnCompleted
      (CallFunction|SetIsEquippingWeapon false))))

(event Custom|FirstShot
  (bind _weaponspread (Variables|Default|GetWeaponSpread))
  ;[1 1 1] Shooting, realoding, ammo
  (Utilities|FlowControl|Sequence
    (:then_0
      (if (and (not (CallFunction|FIsOutOfAmmo)) (not (Variables|Default|GetbIsReloading)))
        (CallFunction|MCWeaponShoot (.ShootingSFX (Utilities|Struct|BreakWeapon_Info (CallFunction|FGetWeaponInfo (Variables|/Game/Blueprints/Weapons/Weapon_Base.Weapon_Base_C|GetWeaponName (stale Custom|SRV_ShootingWeapon Weapon))))) (Transformation|GetActorLocation) (stale Custom|SRV_ShootingWeapon Weapon))
        (CallFunction|FSubtractAmmo 1)))
    (:then_1
      (bind (_outhit _returnvalue) (Collision|LineTraceByChannel (stale Custom|SRV_ShootingWeapon BulletStart) (Math|Vector|MakeVector (Math|Random|RandomFloatinRange (- (.X (Math|Vector|BreakVector (stale Custom|SRV_ShootingWeapon BulletEnd))) _weaponspread) (+ (.X (Math|Vector|BreakVector (stale Custom|SRV_ShootingWeapon BulletEnd))) _weaponspread)) (Math|Random|RandomFloatinRange (- (.Y (Math|Vector|BreakVector (stale Custom|SRV_ShootingWeapon BulletEnd))) _weaponspread) (+ (.Y (Math|Vector|BreakVector (stale Custom|SRV_ShootingWeapon BulletEnd))) _weaponspread)) (Math|Random|RandomFloatinRange (- (.Z (Math|Vector|BreakVector (stale Custom|SRV_ShootingWeapon BulletEnd))) _weaponspread) (+ _weaponspread (.Z (Math|Vector|BreakVector (stale Custom|SRV_ShootingWeapon BulletEnd)))))) "TraceTypeQuery1" false 0 "None"))
      (if _returnvalue
        (if (and (.bBlockingHit (Collision|BreakHitResult _outhit)) (Actor|ActorHasTag (.HitActor (Collision|BreakHitResult _outhit)) "Enemy"))
          (CallFunction|FDamageMultiplier)
          (Game|Damage|ApplyDamage (.HitActor (Collision|BreakHitResult _outhit)) (* (Utilities|Struct|BreakWeapon_Info (CallFunction|FGetWeaponInfo (Variables|/Game/Blueprints/Weapons/Weapon_Base.Weapon_Base_C|GetWeaponName (Variables|Default|GetEquipedWeapon)))) (Variables|Default|GetDamageMultiplier)) 0 0))))
    (:then_2
      (if (and (CallFunction|FIsOutOfAmmo) (not (Variables|Default|GetbIsReloading)))
        (CallFunction|SetIsReloadingWeapon true)))))

(event Custom|CanShootAgain
  ;[1 1 1] Shooting, realoding, ammo
  (Utilities|FlowControl|DoOnce false) ; enters at Reset
)

(event Custom|ShootWeaponLoop
  (bind _weaponspread (Variables|Default|GetWeaponSpread))
  ;[1 1 1] Shooting, realoding, ammo
  (Utilities|FlowControl|Sequence
    (:then_0
      (if (and (not (CallFunction|FIsOutOfAmmo)) (not (Variables|Default|GetbIsReloading)))
        (CallFunction|MCWeaponShoot (.ShootingSFX (Utilities|Struct|BreakWeapon_Info (CallFunction|FGetWeaponInfo (Variables|/Game/Blueprints/Weapons/Weapon_Base.Weapon_Base_C|GetWeaponName (stale Custom|SRV_ShootingWeapon Weapon))))) (Transformation|GetActorLocation) (stale Custom|SRV_ShootingWeapon Weapon))
        (CallFunction|FSubtractAmmo 1)))
    (:then_1
      (bind (_outhit _returnvalue) (Collision|LineTraceByChannel (stale Custom|SRV_ShootingWeapon BulletStart) (Math|Vector|MakeVector (Math|Random|RandomFloatinRange (- (.X (Math|Vector|BreakVector (stale Custom|SRV_ShootingWeapon BulletEnd))) _weaponspread) (+ (.X (Math|Vector|BreakVector (stale Custom|SRV_ShootingWeapon BulletEnd))) _weaponspread)) (Math|Random|RandomFloatinRange (- (.Y (Math|Vector|BreakVector (stale Custom|SRV_ShootingWeapon BulletEnd))) _weaponspread) (+ (.Y (Math|Vector|BreakVector (stale Custom|SRV_ShootingWeapon BulletEnd))) _weaponspread)) (Math|Random|RandomFloatinRange (- (.Z (Math|Vector|BreakVector (stale Custom|SRV_ShootingWeapon BulletEnd))) _weaponspread) (+ _weaponspread (.Z (Math|Vector|BreakVector (stale Custom|SRV_ShootingWeapon BulletEnd)))))) "TraceTypeQuery1" false 0 "None"))
      (if _returnvalue
        (if (and (.bBlockingHit (Collision|BreakHitResult _outhit)) (Actor|ActorHasTag (.HitActor (Collision|BreakHitResult _outhit)) "Enemy"))
          (CallFunction|FDamageMultiplier)
          (Game|Damage|ApplyDamage (.HitActor (Collision|BreakHitResult _outhit)) (* (Utilities|Struct|BreakWeapon_Info (CallFunction|FGetWeaponInfo (Variables|/Game/Blueprints/Weapons/Weapon_Base.Weapon_Base_C|GetWeaponName (Variables|Default|GetEquipedWeapon)))) (Variables|Default|GetDamageMultiplier)) 0 0))))
    (:then_2
      (if (and (CallFunction|FIsOutOfAmmo) (not (Variables|Default|GetbIsReloading)))
        (CallFunction|SetIsReloadingWeapon true)))))

(event Custom|MC_WeaponShoot
  (params (SFX :type Sound%20Base%20Object%20Reference) (Location :type Vector) (Weapon :type Weapon%20Base%20Object%20Reference))
  ;[1 1 1] Shooting, realoding, ammo
  (Animation|Montage|PlayMontage (Variables|Character|GetMesh) (.ShootAnimation (Utilities|Struct|BreakWeapon_Info (CallFunction|FGetWeaponInfo (Variables|/Game/Blueprints/Weapons/Weapon_Base.Weapon_Base_C|GetWeaponName Weapon))))
    (:then
      (Audio|PlaySoundatLocation SFX Location "0, 0, 0" 1.0 1.0 0.0 0 0 0 0))))

(event Custom|SetIsEquippingWeapon
  (params (bIsEquipingWeapon :type Boolean))
  ;[1 1 1] Shooting, realoding, ammo
  (CallFunction|SRVSetIsEquippingWeapon bIsEquipingWeapon))

(event Custom|SRV_SetIsEquippingWeapon
  (params (bIsEquipingWeapon :type Boolean))
  ;[1 1 1] Shooting, realoding, ammo
  (bind _output_get (Variables|Default|SetbIsEquipingWeapon bIsEquipingWeapon))
  (if _output_get
    (CallFunction|MCSwitchWeapon (.EquipAnimation (Utilities|Struct|BreakWeapon_Info (CallFunction|FGetWeaponInfo (Variables|/Game/Blueprints/Weapons/Weapon_Base.Weapon_Base_C|GetWeaponName (Variables|Default|GetEquipedWeapon))))))
    (else
      (Variables|Default|SetbIsReloading false)
      (if (CallFunction|FIsOutOfAmmo)
        (CallFunction|SetIsReloadingWeapon true)))))

(event Custom|SRV_CalculateAimDirection
  ;[1 1 1] Player Movment
  (CallFunction|FCalculateAimDirection))

(event Custom|CL_UpdateAmmoUI
  (params (CurrentAmmo :type Integer) (CurrentReserve :type Integer))
  ;[1 1 1] Shooting, realoding, ammo
  (Default|UpdateAmmoUI (Variables|/Game/Blueprints/Player/IP_PlayerController.IP_PlayerController_C|GetWB_Main (Variables|Default|GetPlayerController)) CurrentAmmo CurrentReserve))

(event Custom|SRV_RandomPlayerLevel
  ;[1 1 1] Player Movment
  (Variables|Default|SetPlayerLevel (Math|Random|RandomIntegerinRange 1 10)))

(event Custom|RandomPlayerLevel
  ;[1 1 1] Player Movment
  (CallFunction|SRVRandomPlayerLevel))

(event Custom|CL_DisplayAmmoUI
  (params (Display :type Boolean))
  ;[1 1 1] Shooting, realoding, ammo
  (Default|DisplayAmmoUI (Variables|/Game/Blueprints/Player/IP_PlayerController.IP_PlayerController_C|GetWB_Main (Variables|Default|GetPlayerController)) Display))

(event Custom|SetIsReloadingWeapon
  (params (bIsReloading :type Boolean))
  ;[1 1 1] Shooting, realoding, ammo
  (CallFunction|SRVSetIsReloadingWeapon bIsReloading))

(event Custom|SRV_SetIsReloadingWeapon
  (params (bIsReloading :type Boolean))
  (bind _equipedweapon (Variables|Default|GetEquipedWeapon))
  (bind _equipedweapon_2 (Variables|Default|GetEquipedWeapon))
  (bind _weaponname (Variables|/Game/Blueprints/Weapons/Weapon_Base.Weapon_Base_C|GetWeaponName _equipedweapon))
  (bind _weaponinfo (CallFunction|FGetWeaponInfo _weaponname))
  (bind (_maxammo _reloadanimation) (Utilities|Struct|BreakWeapon_Info _weaponinfo))
  ;[1 1 1] Shooting, realoding, ammo
  (bind _output_get (Variables|Default|SetbIsReloading bIsReloading))
  (if _output_get
    (CallFunction|MCSetIsReloadingWeapon _reloadanimation)
    (else
      (bind _output_get_2 (Variables|/Game/Blueprints/Weapons/Weapon_Base.Weapon_Base_C|SetCurrentAmmo _equipedweapon_2 _maxammo))
      (CallFunction|CLUpdateAmmoUI _output_get_2 (Variables|/Game/Blueprints/Weapons/Weapon_Base.Weapon_Base_C|GetCurrentReserveAmmo _equipedweapon_2)))))

(event Custom|MC_SetIsReloadingWeapon
  (params (MontageToPlay :type Anim%20Montage%20Object%20Reference))
  ;[1 1 1] Shooting, realoding, ammo
  (Animation|Montage|PlayMontage (Variables|Character|GetMesh) MontageToPlay
    (:OnCompleted
      (CallFunction|SRVSetIsReloadingWeapon false))))

(event Custom|SetPlayerHealth
  (params (CurrentHealth :type Float%20%28double-precision%29))
  (CallFunction|SRVSetPlayerHealth CurrentHealth))

(event Custom|SRV_SetPlayerHealth
  (params (CurrentHealth :type Float%20%28double-precision%29))
  (bind _output_get (Variables|Default|SetCurrentHealth CurrentHealth))
  (CallFunction|CLSetPlayerHealth _output_get (Variables|Default|GetMaxHealth)))

(event Custom|OverlappingWeapons
  (params (Weapon :type Weapon%20Base%20Object%20Reference))
  ;[1 1 1] Equip and Switch
  (CallFunction|SRVOverlappingWeapons Weapon))

(event Custom|CL_SetPlayerHealth
  (params (CurrentHealth :type Float%20%28double-precision%29) (MaxHealth :type Float%20%28double-precision%29))
  (Default|UpdateHealthUI (Variables|/Game/Blueprints/Player/IP_PlayerController.IP_PlayerController_C|GetWB_Main (Variables|Default|GetPlayerController)) CurrentHealth MaxHealth))

(event Custom|HealthRegeneration
  (if (Variables|Default|GetTakenDamge)
    (Utilities|FlowControl|Delay 2.0)
    (Variables|Default|SetTakenDamge false)
    (else
      (Utilities|FlowControl|Delay (Variables|Default|GetHealthRate))
      (if (< (Variables|Default|GetCurrentHealth) (Variables|Default|GetMaxHealth))
        (bind _output_get (Variables|Default|SetCurrentHealth (+ (Variables|Default|GetCurrentHealth) (Variables|Default|GetHealthRegen))))
        (if (>= (Variables|Default|GetCurrentHealth) (Variables|Default|GetMaxHealth))
          (bind _output_get_2 (Variables|Default|SetCurrentHealth 1e+02))
          (CallFunction|CLSetPlayerHealth _output_get_2 (Variables|Default|GetMaxHealth))
          (else
            (CallFunction|CLSetPlayerHealth _output_get (Variables|Default|GetMaxHealth))))))))

(event Custom|SRV_HealthRegenCheck
  (if (not (Variables|Default|GetIsDead))
    (Utilities|Time|SetTimerbyEvent (delegate Custom|HealthRegeneration) 2.0 true)))

(event Custom|Death
  (bind _mesh (Variables|Character|GetMesh))
  (Collision|SetCollisionEnabled (Variables|Collision|GetCapsuleComponent) "NoCollision")
  (Collision|SetCollisionEnabled _mesh "PhysicsOnly")
  (Physics|SetSimulatePhysics _mesh true)
  (Components|Animation|PlayAnimation _mesh 0 false)
  (Pawn|Components|CharacterMovement|DisableMovement (Variables|Character|GetCharacterMovement)))

(event Custom|SRV_WeaponPickup
  (bind _weaponinvent (Variables|Default|GetWeaponInvent))
  (bind _overlappingweapon (Variables|Default|GetOverlappingWeapon))
  (bind _output (Utilities|Array|Get(acopy) _overlappingweapon))
  ;[1 1 1] Equip and Switch
  (if (Utilities|Array|IsNotEmpty _overlappingweapon)
    (Utilities|Array|SetArrayElem _weaponinvent (Utilities|Array|Length _weaponinvent) _output true)
    (if (== _output (Variables|Default|GetPickedUpWeapon))
      (Variables|Default|SetPickedUpWeapon 0))
    (bind _output_get (Variables|Default|SetPickedUpWeapon _output))
    (Utilities|FlowControl|Delay 0.05)
    (if (Utilities|Enum|Equal(Enum) (Variables|Default|GetEquippedWeapon) "NewEnumerator0")
      (Variables|Default|SetEquipedWeapon _output_get)
      (Utilities|FlowControl|Delay 0.05)
      (CallFunction|SetEquipedWeapon (.WeaponType (Utilities|Struct|BreakWeapon_Info (CallFunction|FGetWeaponInfo (Variables|/Game/Blueprints/Weapons/Weapon_Base.Weapon_Base_C|GetWeaponName (Variables|Default|GetPickedUpWeapon))))))
      (CallFunction|SetIsEquippingWeapon true)
      (CallFunction|CLUpdateAmmoUI (Variables|/Game/Blueprints/Weapons/Weapon_Base.Weapon_Base_C|GetCurrentAmmo (Variables|Default|GetEquipedWeapon)) (Variables|/Game/Blueprints/Weapons/Weapon_Base.Weapon_Base_C|GetCurrentReserveAmmo (Variables|Default|GetEquipedWeapon)))
      (CallFunction|CLDisplayAmmoUI true)
      (Variables|Default|SetPickedUpWeapon 0)
      (Utilities|Array|RemoveItem (Variables|Default|GetOverlappingWeapon) _output)
      (CallFunction|CheckforMoreOverlapping))
    (else
      (CallFunction|CanPickUpAgain))))

(event Custom|SRV_OverlappingWeapons
  (params (Weapon :type Weapon%20Base%20Object%20Reference))
  (bind _overlappingweapon (Variables|Default|GetOverlappingWeapon))
  ;[1 1 1] Equip and Switch
  (Utilities|Array|SetArrayElem _overlappingweapon (Utilities|Array|Length _overlappingweapon) Weapon true)
  (Utilities|FlowControl|DoOnce false
    (:Completed
      (CallFunction|WeaponPickUp))))

(event Custom|SetEquipedWeapon
  (params (EquippedWeapon :type Weapon_Type%20Enum :default "NewEnumerator0"))
  ;[1 1 1] Equip and Switch
  (CallFunction|SRVSetEquipedWeapon EquippedWeapon))

(event Custom|CheckForMoreOverlapping
  ;[1 1 1] Equip and Switch
  (CallFunction|WeaponPickUp))

(event Custom|SRV_SetEquipedWeapon
  (params (EquippedWeapon :type Weapon_Type%20Enum :default "NewEnumerator0"))
  ;[1 1 1] Equip and Switch
  (Variables|Default|SetEquippedWeapon EquippedWeapon))

(event Custom|WeaponPickUp
  ;[1 1 1] Equip and Switch
  (CallFunction|SRVWeaponPickup))

(event Input|EnhancedActionEvents|EnhancedInputActionMovement_Action
  (params (ActionValue :type Vector%202D%20Structure) (ElapsedSeconds :type Float%20%28double-precision%29) (TriggeredSeconds :type Float%20%28double-precision%29) (InputAction :type Input%20Action%20Object%20Reference :default "/Game/Blueprints/Player/Inputs/Movement_Action.Movement_Action"))
  ;[1 1 1] Player Movment
  (Pawn|Input|AddMovementInput (Transformation|GetActorForwardVector) (.x ActionValue) false)
  (Pawn|Input|AddMovementInput (Transformation|GetActorRightVector) (.y ActionValue) false))

(event Input|EnhancedActionEvents|EnhancedInputActionMouse_Movement
  (params (ActionValue :type Vector%202D%20Structure) (ElapsedSeconds :type Float%20%28double-precision%29) (TriggeredSeconds :type Float%20%28double-precision%29) (InputAction :type Input%20Action%20Object%20Reference :default "/Game/Blueprints/Player/Inputs/Mouse_Movement.Mouse_Movement"))
  ;[1 1 1] Player Movment
  (Pawn|Input|AddControllerYawInput (.x ActionValue))
  (Pawn|Input|AddControllerPitchInput (.y ActionValue))
  (CallFunction|FCalculateAimDirection))

(event Input|EnhancedActionEvents|EnhancedInputActionCrouch
  (params (ActionValue :type Boolean) (ElapsedSeconds :type Float%20%28double-precision%29) (TriggeredSeconds :type Float%20%28double-precision%29) (InputAction :type Input%20Action%20Object%20Reference :default "/Game/Blueprints/Player/Inputs/Crouch.Crouch"))
  ;[1 1 1] Player Movment
  (if (CallFunction|FIsNotJumping) :!label _label
    (if ActionValue
      (CallFunction|FCrouch true)
      (else
        (CallFunction|FCrouch false)))
    (else
      (Utilities|FlowControl|Delay 0.05)
      (goto _label))))

(event Input|EnhancedActionEvents|EnhancedInputActionWalk
  (params (ActionValue :type Boolean) (ElapsedSeconds :type Float%20%28double-precision%29) (TriggeredSeconds :type Float%20%28double-precision%29) (InputAction :type Input%20Action%20Object%20Reference :default "/Game/Blueprints/Player/Inputs/Walk.Walk"))
  ;[1 1 1] Player Movment
  (if ActionValue
    (CallFunction|FWalk true)
    (else
      (CallFunction|FWalk false))))

(event Input|EnhancedActionEvents|EnhancedInputActionJump
  (params (ActionValue :type Boolean) (ElapsedSeconds :type Float%20%28double-precision%29) (TriggeredSeconds :type Float%20%28double-precision%29) (InputAction :type Input%20Action%20Object%20Reference :default "/Game/Blueprints/Player/Inputs/Jump.Jump"))
  ;[1 1 1] Player Movment
  (if (CallFunction|FIsNotJumping)
    (Character|Jump)))

(event Input|EnhancedActionEvents|EnhancedInputActionShoot_Weapon
  (params (ActionValue :type Boolean) (ElapsedSeconds :type Float%20%28double-precision%29) (TriggeredSeconds :type Float%20%28double-precision%29) (InputAction :type Input%20Action%20Object%20Reference :default "/Game/Blueprints/Player/Inputs/Shoot_Weapon.Shoot_Weapon"))
  (bind (_bulletstart _bulletend) (CallFunction|FGetLineTrace))
  ;[1 1 1] Shooting, realoding, ammo
  (:Triggered
    (if (Math|Boolean|ANDBoolean (Utilities|Enum|NotEqual(Enum) (Variables|Default|GetEquippedWeapon) "NewEnumerator0") (not (Variables|Default|GetbIsEquipingWeapon)) (not (Variables|Default|GetbIsReloading)))
      (bind _equipedweapon (Variables|Default|GetEquipedWeapon)
        (:then
          (CallFunction|SRVShootingWeapon _equipedweapon true _bulletstart _bulletend))
        (:else))
      (else
        (CallFunction|SRVShootingWeapon _equipedweapon false "0, 0, 0" "0, 0, 0" :!label _label))))
  (:Completed
    (goto _label)))

(event Input|EnhancedActionEvents|EnhancedInputActionPrimary_Weapon
  (params (ActionValue :type Boolean) (ElapsedSeconds :type Float%20%28double-precision%29) (TriggeredSeconds :type Float%20%28double-precision%29) (InputAction :type Input%20Action%20Object%20Reference :default "/Game/Blueprints/Player/Inputs/Primary_Weapon.Primary_Weapon"))
  ;[1 1 1] Equip and Switch
  (if (Utilities|Enum|NotEqual(Enum) (Variables|Default|GetEquippedWeapon) "NewEnumerator2")
    (CallFunction|SRVSwitchWeapon "NewEnumerator2")))

(event Input|EnhancedActionEvents|EnhancedInputActionSecondary_Weapon
  (params (ActionValue :type Boolean) (ElapsedSeconds :type Float%20%28double-precision%29) (TriggeredSeconds :type Float%20%28double-precision%29) (InputAction :type Input%20Action%20Object%20Reference :default "/Game/Blueprints/Player/Inputs/Secondary_Weapon.Secondary_Weapon"))
  ;[1 1 1] Equip and Switch
  (if (Utilities|Enum|NotEqual(Enum) (Variables|Default|GetEquippedWeapon) "NewEnumerator1")
    (CallFunction|SRVSwitchWeapon "NewEnumerator1")))

(event Input|EnhancedActionEvents|EnhancedInputActionReload_Weapon
  (params (ActionValue :type Boolean) (ElapsedSeconds :type Float%20%28double-precision%29) (TriggeredSeconds :type Float%20%28double-precision%29) (InputAction :type Input%20Action%20Object%20Reference :default "/Game/Blueprints/Player/Inputs/Reload_Weapon.Reload_Weapon"))
  ;[1 1 1] Shooting, realoding, ammo
  (Variables|Default|GetEquipedWeapon
    (:then
      (if (Math|Boolean|ANDBoolean (!= (Variables|/Game/Blueprints/Weapons/Weapon_Base.Weapon_Base_C|GetCurrentAmmo (Variables|Default|GetEquipedWeapon)) (.MaxAmmo (Utilities|Struct|BreakWeapon_Info (CallFunction|FGetWeaponInfo (Variables|/Game/Blueprints/Weapons/Weapon_Base.Weapon_Base_C|GetWeaponName (Variables|Default|GetEquipedWeapon)))))) (Utilities|Enum|NotEqual(Enum) (Variables|Default|GetEquippedWeapon) "NewEnumerator0") (not (Variables|Default|GetbIsReloading)))
        (CallFunction|SetIsReloadingWeapon true)))
    (:else)))

(event Input|EnhancedActionEvents|EnhancedInputActionPauseMenu
  (params (ActionValue :type Boolean) (ElapsedSeconds :type Float%20%28double-precision%29) (TriggeredSeconds :type Float%20%28double-precision%29) (InputAction :type Input%20Action%20Object%20Reference :default "/Game/Blueprints/Player/Inputs/PauseMenu.PauseMenu"))
  ;[1 1 1] Player Movment
  (bind _returnvalue (Game|GetCurrentLevelName true))
  (if (Utilities|Enum|Equal(Enum) _returnvalue "Play_Level")
    (Default|PauseMenu (Variables|Default|GetPlayerController))))

(event Game|Damage|EventAnyDamage
  (params (Damage :type Float%20%28single-precision%29) (DamageType :type Damage%20Type%20Object%20Reference) (InstigatedBy :type Controller%20Object%20Reference) (DamageCauser :type Actor%20Object%20Reference))
  (Variables|Default|SetTakenDamge true)
  (CallFunction|SetPlayerHealth (Math|Float|Clamp(Float) (- (Variables|Default|GetCurrentHealth) Damage) 0.0 (Variables|Default|GetMaxHealth))))

(event EventBeginPlay
  ;[1 1 1] Player Movment
  (bind _playercontroller (Class|INTPlayerController|GetPlayerControllerRef(Message) (Pawn|GetController)))
  (Utilities|IsValid _playercontroller
    (:Is%20Valid
      (Variables|Default|SetPlayerController _playercontroller)
      (Input|AddMappingContext (PlayerController|LocalPlayerSubsystems|GetEnhancedInputLocalPlayerSubsystem _playercontroller) "/Game/Blueprints/Player/Inputs/Default.Default" 0 "(bIgnoreAllPressedKeysUntilRelease=True,bForceImmediately=False,bNotifyUserSettings=False)")
      (CallFunction|RandomPlayerLevel)
      (bind _returnvalue (Game|GetCurrentLevelName true))
      (if (Utilities|Enum|Equal(Enum) _returnvalue "Play_Level")
        (CallFunction|SetPlayerHealth (Variables|Default|GetMaxHealth))
        (Utilities|FlowControl|Delay 0.2)
        (CallFunction|SRVHealthRegenCheck)))))

(fn ConstructionScript)

(fn FCrouch
  (params (bCrouch :type Boolean))
  (bind _output_get (LocalVariables|SetCrouch%20Local bCrouch))
  (Networking|SwitchHasAuthority
    (:Authority
      _)
    (:Remote
      (CallFunction|SRVCrouch _output_get)))
  (if (LocalVariables|GetCrouch%20Local)
    (Character|Crouch)
    (Variables|Default|SetbCrouch true)
    (else
      (Character|UnCrouch)
      (Variables|Default|SetbCrouch false))))

(fn FWalk
  (params (bWalk :type Boolean))
  (bind _output_get (LocalVariables|SetWalk%20Local bWalk))
  (Networking|SwitchHasAuthority
    (:Authority
      _)
    (:Remote
      (CallFunction|SRVWalk _output_get)))
  (if (LocalVariables|GetWalk%20Local)
    (Variables|/Script/Engine.CharacterMovementComponent|SetMaxWalkSpeed (Variables|Character|GetCharacterMovement) (Variables|Default|GetWalk%20Speed))
    (Variables|Default|SetbWalk true)
    (else
      (Variables|/Script/Engine.CharacterMovementComponent|SetMaxWalkSpeed (Variables|Character|GetCharacterMovement) (Variables|Default|GetRun%20Speed))
      (Variables|Default|SetbWalk false))))

(fn FIsNotJumping
  (return (not (AI|Components|NavMovement|IsFalling (Variables|Character|GetCharacterMovement)))))

(fn FCalculateAimDirection
  (Networking|SwitchHasAuthority
    (:Authority
      _)
    (:Remote
      (CallFunction|SRVCalculateAimDirection)))
  (Variables|Default|SetAimDirection (.Pitch (Math|Rotator|BreakRotator (Math|Rotator|Delta(Rotator) (Pawn|GetControlRotation :!class /Script/Engine.Pawn) (Transformation|GetActorRotation))))))

(fn OnRepPickedUpWeapon
  (bind _pickedupweapon (Variables|Default|GetPickedUpWeapon))
  (bind _pickedupweapon_2 (Variables|Default|GetPickedUpWeapon)
    (:then
      (Physics|SetSimulatePhysics (Variables|/Game/Blueprints/Weapons/Weapon_Base.Weapon_Base_C|GetWeapon _pickedupweapon_2) false)
      (Collision|SetCollisionEnabled (Variables|/Game/Blueprints/Weapons/Weapon_Base.Weapon_Base_C|GetWeapon _pickedupweapon_2) "NoCollision")
      (Collision|SetCollisionEnabled (Variables|/Game/Blueprints/Weapons/Weapon_Base.Weapon_Base_C|GetCollisionSphere (Variables|Default|GetPickedUpWeapon)) "NoCollision")
      (Transformation|AttachComponentToComponent (Variables|/Game/Blueprints/Weapons/Weapon_Base.Weapon_Base_C|GetWeapon _pickedupweapon) (Variables|/Game/Blueprints/Weapons/Weapon_Base.Weapon_Base_C|GetDefaultSceneRoot _pickedupweapon) "None" "SnapToTarget" "SnapToTarget" "SnapToTarget" true)
      (if (Utilities|Enum|Equal(Enum) (Variables|Default|GetEquippedWeapon) "NewEnumerator0")
        (Transformation|AttachComponentToComponent (Variables|/Game/Blueprints/Weapons/Weapon_Base.Weapon_Base_C|GetWeapon (Variables|Default|GetPickedUpWeapon)) (Variables|Character|GetMesh) (Utilities|Select :Index (.WeaponType (Utilities|Struct|BreakWeapon_Info (CallFunction|FGetWeaponInfo (Variables|/Game/Blueprints/Weapons/Weapon_Base.Weapon_Base_C|GetWeaponName (Variables|Default|GetPickedUpWeapon))))) :NewEnumerator0 "None" :NewEnumerator1 "S_Pistol" :NewEnumerator2 "S_Rifle") "SnapToTarget" "SnapToTarget" "SnapToTarget" true)
        (else
          (Transformation|AttachComponentToComponent (Variables|/Game/Blueprints/Weapons/Weapon_Base.Weapon_Base_C|GetWeapon (Variables|Default|GetPickedUpWeapon)) (Variables|Character|GetMesh) (Utilities|Select :Index (.WeaponType (Utilities|Struct|BreakWeapon_Info (CallFunction|FGetWeaponInfo (Variables|/Game/Blueprints/Weapons/Weapon_Base.Weapon_Base_C|GetWeaponName (Variables|Default|GetPickedUpWeapon))))) :NewEnumerator0 "None" :NewEnumerator1 "S_WeaponSide" :NewEnumerator2 "S_WeaponBack") "SnapToTarget" "SnapToTarget" "SnapToTarget" true))))
    (:else)))

(fn OnRepEquipWeapon
  (bind _equipweapon (Variables|Default|GetEquipWeapon)
    (:then
      (Transformation|AttachComponentToComponent (Variables|/Game/Blueprints/Weapons/Weapon_Base.Weapon_Base_C|GetWeapon _equipweapon) (Variables|Character|GetMesh) (Utilities|Select :Index (.WeaponType (Utilities|Struct|BreakWeapon_Info (CallFunction|FGetWeaponInfo (Variables|/Game/Blueprints/Weapons/Weapon_Base.Weapon_Base_C|GetWeaponName (Variables|Default|GetEquipWeapon))))) :NewEnumerator0 "None" :NewEnumerator1 "S_Pistol" :NewEnumerator2 "S_Rifle") "SnapToTarget" "SnapToTarget" "SnapToTarget" true))
    (:else)))

(fn OnRepUnequipWeapon
  (bind _unequipweapon (Variables|Default|GetUnequipWeapon)
    (:then
      (Transformation|AttachComponentToComponent (Variables|/Game/Blueprints/Weapons/Weapon_Base.Weapon_Base_C|GetWeapon _unequipweapon) (Variables|Character|GetMesh) (Utilities|Select :Index (.WeaponType (Utilities|Struct|BreakWeapon_Info (CallFunction|FGetWeaponInfo (Variables|/Game/Blueprints/Weapons/Weapon_Base.Weapon_Base_C|GetWeaponName (Variables|Default|GetUnequipWeapon))))) :NewEnumerator0 "None" :NewEnumerator1 "S_WeaponSide" :NewEnumerator2 "S_WeaponBack") "SnapToTarget" "SnapToTarget" "SnapToTarget" true))
    (:else)))

(fn FGetLineTrace
  (bind _playercontroller (Class|INTPlayerController|GetPlayerControllerRef(Message) (Pawn|GetController)))
  (return (Camera|GetCameraLocation (Variables|/Script/Engine.PlayerController|GetPlayerCameraManager _playercontroller)) (+ (Camera|GetCameraLocation (Variables|/Script/Engine.PlayerController|GetPlayerCameraManager _playercontroller)) (* (Transformation|GetActorForwardVector (Variables|/Script/Engine.PlayerController|GetPlayerCameraManager _playercontroller)) 20000))))

(fn FSubtractAmmo
  (params (AmmoToSubstract :type Integer))
  (bind _equipedweapon (Variables|Default|GetEquipedWeapon))
  (bind _currentreserveammo (Variables|/Game/Blueprints/Weapons/Weapon_Base.Weapon_Base_C|GetCurrentReserveAmmo _equipedweapon))
  (bind _output_get (Variables|/Game/Blueprints/Weapons/Weapon_Base.Weapon_Base_C|SetCurrentAmmo _equipedweapon (Math|Integer|Clamp(Integer) (- (Variables|/Game/Blueprints/Weapons/Weapon_Base.Weapon_Base_C|GetCurrentAmmo _equipedweapon) AmmoToSubstract) 0 _currentreserveammo)))
  (CallFunction|CLUpdateAmmoUI _output_get _currentreserveammo))

(fn FIsOutOfAmmo
  (return (== (Variables|/Game/Blueprints/Weapons/Weapon_Base.Weapon_Base_C|GetCurrentAmmo (Variables|Default|GetEquipedWeapon)) 0)))

(fn FDamageMultiplier
  (switch int (Variables|Default|GetPlayerLevel)
    (:1
      (Variables|Default|SetDamageMultiplier 1.0))
    (:2
      (Variables|Default|SetDamageMultiplier 1.2))
    (:3
      (Variables|Default|SetDamageMultiplier 1.3))
    (:4
      (Variables|Default|SetDamageMultiplier 1.4))
    (:5
      (Variables|Default|SetDamageMultiplier 1.5))
    (:6
      (Variables|Default|SetDamageMultiplier 1.6))
    (:7
      (Variables|Default|SetDamageMultiplier 1.7))
    (:8
      (Variables|Default|SetDamageMultiplier 1.8))
    (:9
      (Variables|Default|SetDamageMultiplier 1.9))
    (:10
      (Variables|Default|SetDamageMultiplier 2.0))))

(fn GetPlayerBaseRef
  (return self))