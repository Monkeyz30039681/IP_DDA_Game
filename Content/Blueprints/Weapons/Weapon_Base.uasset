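; Base weapon pickup actor that simulates physics in the world and offers itself to players who overlap it.
; An initialise event on BeginPlay fills current and reserve ammo from weapon info looked up by name.
; On authority, sphere overlap compares weapon type against the player's inventory, stopping at the first differing type.
; A match blocks looting and resets the flag; otherwise the weapon passes itself to the player's OverlappingWeapons.
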(event OnComponentBeginOverlap(CollisionSphere)
  (params (OverlappedComponent :type Primitive%20Component%20Object%20Reference) (OtherActor :type Actor%20Object%20Reference) (OtherComp :type Primitive%20Component%20Object%20Reference) (OtherBodyIndex :type Integer) (bFromSweep :type Boolean) (SweepResult :type Hit%20Result%20Structure%20%28by%20ref%29))
  (if (Actor|ActorHasTag OtherActor "Player")
    (Networking|SwitchHasAuthority
      (:Authority
        (bind _player (Class|INTPlayerBase|GetPlayerBaseRef(Message) OtherActor))
        (bind _array_element (Utilities|Array|ForEachLoopwithBreak (Variables|/Game/Blueprints/Player/Player_Charcter_Base.Player_Charcter_Base_C|GetWeaponInvent _player) :!label _label)
          (:LoopBody
            (if (Utilities|Enum|Equal(Enum) (.WeaponType (Utilities|Struct|BreakWeapon_Info (CallFunction|FGetWeaponInfo (Variables|Weapon_Base_C|GetWeaponName _array_element)))) (.WeaponType (Utilities|Struct|BreakWeapon_Info (CallFunction|FGetWeaponInfo (Variables|Default|GetWeaponName)))))
              (Variables|/Game/Blueprints/Player/Player_Charcter_Base.Player_Charcter_Base_C|SetbCanLootWeapon _player false)
              (else
                (goto _label Break))))
          (:Completed
            (if (Variables|/Game/Blueprints/Player/Player_Charcter_Base.Player_Charcter_Base_C|GetbCanLootWeapon _player)
              (Default|OverlappingWeapons _player self)
              (else
                (Variables|/Game/Blueprints/Player/Player_Charcter_Base.Player_Charcter_Base_C|SetbCanLootWeapon _player true)))))))))

(event Custom|SRV_InitialiseWeapon
  (bind _weaponname (Variables|Default|GetWeaponName))
  (bind _weaponinfo (CallFunction|FGetWeaponInfo _weaponname))
  (bind (_maxammo _reserveammo) (Utilities|Struct|BreakWeapon_Info _weaponinfo))
  (Variables|Default|SetCurrentAmmo _maxammo)
  (Variables|Default|SetCurrentReserveAmmo _reserveammo))

(event EventBeginPlay
  (Physics|SetSimulatePhysics (Variables|Default|GetWeapon) true)
  (CallFunction|SRVInitialiseWeapon))

(fn ConstructionScript)