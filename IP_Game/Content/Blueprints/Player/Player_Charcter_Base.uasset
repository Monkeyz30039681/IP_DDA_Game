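; Base multiplayer player character handling movement, aim pitch and a weapon inventory with pickup, drop and rifle/pistol switching.
; Enhanced Input drives locomotion and server RPCs; crouch, walk and aim run locally and are forwarded to the server.
; Overlapped weapons queue for looting, pickup drops any same-type weapon, and a macro searches inventory by type.
; RepNotifies handle socket attachment and drop physics, multicast plays equip montages, and shooting is an empty stub.
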(event Custom|SRV_Crouch
  (params (bCrouch :type Boolean))
  ;[1 1 1] Player Movment
  (CallFunction|FCrouch bCrouch))

(event Custom|SRV_Walk
  (params (bWalk :type Boolean))
  ;[1 1 1] Player Movment
  (CallFunction|FWalk bWalk))

(event Custom|CanLootWeaponAgain
  ;[1 1 1] Weapon drop and pickup
  (Utilities|FlowControl|DoOnce false) ; enters at Reset
)

(event Custom|SRV_DropWeapon
  ;[1 1 1] Weapon drop and pickup
  (bind (_weaponfound _weapon) (Utilities|MFindWeaponTypeinInventory (Variables|Default|GetEquippedWeapon) :!label _label)
    (:LoopBody
      (if _weaponfound
        (CallFunction|FDropWeapon _weapon)
        (goto _label Break%20Loop)))
    (:LoopCompleted
      (Utilities|FlowControl|Delay 0.1)
      (Variables|/Game/Blueprints/Weapons/Weapon_Base.Weapon_Base_C|SetbCanBeInteractedWith (Variables|Default|GetWeaponToDrop) true)
      (Variables|Default|SetWeaponToDrop 0))))

(event Custom|SetDroppedWeapon
  (params (DroppedWeapon :type Weapon%20Base%20Object%20Reference))
  ;[1 1 1] Weapon drop and pickup
  (CallFunction|SRVSetDroppedWeapon DroppedWeapon))

(event Custom|SRV_SetDroppedWeapon
  (params (DroppedWeapon :type Weapon%20Base%20Object%20Reference))
  ;[1 1 1] Weapon drop and pickup
  (Variables|Default|SetDropped%20Weapon DroppedWeapon))

(event Custom|SRV_ResquestPickupWeapon
  (bind _overlappingactors (Collision|GetOverlappingActors "/Game/Blueprints/Weapons/Weapon_Base.Weapon_Base_C" :!class /Script/Engine.Actor))
  ;[1 1 1] Weapon drop and pickup
  (if (Utilities|Array|IsNotEmpty _overlappingactors)
    (bind (_weaponfound _weapon) (Utilities|MFindWeaponTypeinInventory (.WeaponType (Utilities|Struct|BreakWeapon_Info (CallFunction|FGetWeaponInfo (Variables|/Game/Blueprints/Weapons/Weapon_Base.Weapon_Base_C|GetWeaponName (stale _weapon_2))))) :!label _label)
      (:LoopBody
        (bind _weapon_2 (Class|INTWeaponBase|GetWeaponRef(Message) (Utilities|Array|Get(acopy) _overlappingactors)))
        (if _weaponfound
          (CallFunction|FDropWeapon _weapon))
        (CallFunction|AddOverlappedItem _weapon_2)
        (goto _label Break%20Loop))
      (:LoopCompleted
        (Utilities|FlowControl|Delay 0.1)
        (bind _weapontodrop (Variables|Default|GetWeaponToDrop)
          (:then
            (Variables|/Game/Blueprints/Weapons/Weapon_Base.Weapon_Base_C|SetbCanBeInteractedWith _weapontodrop true)
            (Variables|Default|SetWeaponToDrop 0))
          (:else))))))

(event Custom|SRV_EquipWeapon
  (params (WeaponTypeToFind :type Weapon_Type%20Enum :default "NewEnumerator0"))
  ;[1 1 1] Switching Weapon
  (bind (_weaponfound _weapon) (Utilities|MFindWeaponTypeinInventory WeaponTypeToFind :!label _label)
    (:LoopBody
      (if _weaponfound
        (Variables|Default|SetbWeaponFoundInInvetory true)
        (goto _label Break%20Loop)))
    (:LoopCompleted
      (if (Variables|Default|GetbWeaponFoundInInvetory)
        (if (Utilities|Enum|Equal(Enum) (Variables|Default|GetEquippedWeapon) "NewEnumerator0")
          (Variables|Default|SetEquipWeapon _weapon :!label _label_2)
          (CallFunction|SetEquippedWeapon WeaponTypeToFind)
          (CallFunction|MCEquipWeapon (Utilities|Struct|BreakWeapon_Info (CallFunction|FGetWeaponInfo (Variables|/Game/Blueprints/Weapons/Weapon_Base.Weapon_Base_C|GetWeaponName (Variables|Default|GetEquipWeapon)))))
          (Variables|Default|SetEquipWeapon 0)
          (Variables|Default|SetUnequipWeapon 0)
          (Variables|Default|SetbWeaponFoundInInvetory false)
          (else
            (bind (_weaponfound_2 _weapon_2) (Utilities|MFindWeaponTypeinInventory (Variables|Default|GetEquippedWeapon) :!label _label_3)
              (:LoopBody
                (if _weaponfound_2
                  (Variables|Default|SetUnequipWeapon _weapon_2)
                  (goto _label_3 Break%20Loop)))
              (:LoopCompleted
                (goto _label_2)))))))))

(event Custom|MC_EquipWeapon
  (params (Equip%20Animation :type Anim%20Montage%20Object%20Reference))
  ;[1 1 1] Switching Weapon
  (Animation|Montage|PlayMontage (Variables|Character|GetMesh) Equip%20Animation))

(event Custom|SRV_CalculateAimDirection
  ;[1 1 1] Player Movment
  (CallFunction|FCalculateAimDirection))

(event Custom|LootWeapon
  ;[1 1 1] Weapon drop and pickup
  (CallFunction|SRVLootWeapon))

(event Custom|SRV_LootWeapon
  (bind _weaponinventory (Variables|Default|GetWeaponInventory))
  (bind _overlappedweapons (Variables|Default|GetOverlappedWeapons))
  (bind _output (Utilities|Array|Get(acopy) _overlappedweapons))
  ;[1 1 1] Weapon drop and pickup
  (Variables|Default|SetbPickingUpWeapon true)
  (if (Utilities|Array|IsNotEmpty _overlappedweapons)
    (Utilities|Array|SetArrayElem _weaponinventory (Utilities|Array|Length _weaponinventory) _output true)
    (Variables|Default|SetLooted%20Weapon _output)
    (if (Utilities|Enum|Equal(Enum) (Variables|Default|GetEquippedWeapon) "NewEnumerator0")
      (Utilities|FlowControl|Delay 0.1)
      (CallFunction|SetEquippedWeapon (.WeaponType (Utilities|Struct|BreakWeapon_Info (CallFunction|FGetWeaponInfo (Variables|/Game/Blueprints/Weapons/Weapon_Base.Weapon_Base_C|GetWeaponName (Variables|Default|GetLooted%20Weapon))))))
      (CallFunction|MCEquipWeapon (.EquipAnimation (Utilities|Struct|BreakWeapon_Info (CallFunction|FGetWeaponInfo (Variables|/Game/Blueprints/Weapons/Weapon_Base.Weapon_Base_C|GetWeaponName (Variables|Default|GetLooted%20Weapon))))))
      (Variables|Default|SetLooted%20Weapon 0))
    (Utilities|Array|RemoveItem (Variables|Default|GetOverlappedWeapons) _output)
    (CallFunction|CheckforOverlappedWeapons)
    (else
      (CallFunction|CanLootWeaponAgain)
      (Variables|Default|SetbPickingUpWeapon false))))

(event Custom|SetEquippedWeapon
  (params (EquippedWeapon :type Weapon_Type%20Enum :default "NewEnumerator0"))
  ;[1 1 1] Weapon drop and pickup
  (CallFunction|SRVSetEquippedWeapon EquippedWeapon))

(event Custom|SRV_SetEquippedWeapon
  (params (EquippedWeapon :type Weapon_Type%20Enum :default "NewEnumerator0"))
  ;[1 1 1] Weapon drop and pickup
  (Variables|Default|SetEquippedWeapon EquippedWeapon))

(event Custom|AddOverlappedItem
  (params (Weapon :type Weapon%20Base%20Object%20Reference))
  ;[1 1 1] Weapon drop and pickup
  (CallFunction|SRVAddOverlappedItem Weapon))

(event Custom|SRV_AddOverlappedItem
  (params (Weapon :type Weapon%20Base%20Object%20Reference))
  (bind _overlappedweapons (Variables|Default|GetOverlappedWeapons))
  ;[1 1 1] Weapon drop and pickup
  (Utilities|Array|SetArrayElem _overlappedweapons (Utilities|Array|Length _overlappedweapons) Weapon true)
  (Utilities|FlowControl|DoOnce false
    (:Completed
      (CallFunction|LootWeapon))))

(event Custom|CheckForOverlappedWeapons
  ;[1 1 1] Weapon drop and pickup
  (CallFunction|LootWeapon))

(event Input|EnhancedActionEvents|EnhancedInputActionMovement_Action
  (params (ActionValue :type Vector%202D%20Structure) (ElapsedSeconds :type Float%20%28double-precision%29) (TriggeredSeconds :type Float%20%28double-precision%29) (InputAction :type Input%20Action%20Object%20Reference :default "/Game/Blueprints/Player/Inputs/Movement_Action.Movement_Action"))
  ;[1 1 1] Player Movment
  (Pawn|Input|AddMovementInput (Transformation|GetActorForwardVector) (.x ActionValue) false)
  (Pawn|Input|AddMovementInput (Transformation|GetActorRightVector) (.y ActionValue) false))

(event Input|EnhancedActionEvents|EnhancedInputActionMouse_Movement
  (params (ActionValue :type Vector%202D%20Structure) (ElapsedSeconds :type Float%20%28double-precision%29) (TriggeredSeconds :type Float%20%28double-precision%29) (InputAction :type Input%20Action%20Object%20Reference :default "/Game/Blueprints/Player/Inputs/Mouse_Movement.Mouse_Movement"))
  ;[1 1 1] Player Movment
  (Pawn|Input|AddControllerYawInput (.x ActionValue))
  (Pawn|Input|AddControllerPitchInput (.y ActionValue))
  (CallFunction|FCalculateAimDirection))

(event Input|EnhancedActionEvents|EnhancedInputActionCrouch
  (params (ActionValue :type Boolean) (ElapsedSeconds :type Float%20%28double-precision%29) (TriggeredSeconds :type Float%20%28double-precision%29) (InputAction :type Input%20Action%20Object%20Reference :default "/Game/Blueprints/Player/Inputs/Crouch.Crouch"))
  ;[1 1 1] Player Movment
  (if (CallFunction|FIsNotJumping) :!label _label
    (if ActionValue
      (CallFunction|FCrouch true)
      (else
        (CallFunction|FCrouch false)))
    (else
      (Utilities|FlowControl|Delay 0.05)
      (goto _label))))

(event Input|EnhancedActionEvents|EnhancedInputActionWalk
  (params (ActionValue :type Boolean) (ElapsedSeconds :type Float%20%28double-precision%29) (TriggeredSeconds :type Float%20%28double-precision%29) (InputAction :type Input%20Action%20Object%20Reference :default "/Game/Blueprints/Player/Inputs/Walk.Walk"))
  ;[1 1 1] Player Movment
  (if ActionValue
    (CallFunction|FWalk true)
    (else
      (CallFunction|FWalk false))))

(event Input|EnhancedActionEvents|EnhancedInputActionJump
  (params (ActionValue :type Boolean) (ElapsedSeconds :type Float%20%28double-precision%29) (TriggeredSeconds :type Float%20%28double-precision%29) (InputAction :type Input%20Action%20Object%20Reference :default "/Game/Blueprints/Player/Inputs/Jump.Jump"))
  ;[1 1 1] Player Movment
  (if (CallFunction|FIsNotJumping)
    (Character|Jump)))

(event Input|EnhancedActionEvents|EnhancedInputActionDrop_Weapon
  (params (ActionValue :type Boolean) (ElapsedSeconds :type Float%20%28double-precision%29) (TriggeredSeconds :type Float%20%28double-precision%29) (InputAction :type Input%20Action%20Object%20Reference :default "/Game/Blueprints/Player/Inputs/Drop_Weapon.Drop_Weapon"))
  ;[1 1 1] Weapon drop and pickup
  (if (Utilities|Enum|NotEqual(Enum) (Variables|Default|GetEquippedWeapon) "NewEnumerator0")
    (CallFunction|SRVDropWeapon)))

(event Input|EnhancedActionEvents|EnhancedInputActionPickup_Weapon
  (params (ActionValue :type Boolean) (ElapsedSeconds :type Float%20%28double-precision%29) (TriggeredSeconds :type Float%20%28double-precision%29) (InputAction :type Input%20Action%20Object%20Reference :default "/Game/Blueprints/Player/Inputs/Pickup_Weapon.Pickup_Weapon"))
  ;[1 1 1] Weapon drop and pickup
  (if (not (Variables|Default|GetbPickingUpWeapon))
    (CallFunction|SRVResquestPickupWeapon)))

(event Input|EnhancedActionEvents|EnhancedInputActionPrimary_Weapon
  (params (ActionValue :type Boolean) (ElapsedSeconds :type Float%20%28double-precision%29) (TriggeredSeconds :type Float%20%28double-precision%29) (InputAction :type Input%20Action%20Object%20Reference :default "/Game/Blueprints/Player/Inputs/Primary_Weapon.Primary_Weapon"))
  ;[1 1 1] Switching Weapon
  (if (Utilities|Enum|NotEqual(Enum) (Variables|Default|GetEquippedWeapon) "NewEnumerator2")
    (CallFunction|SRVEquipWeapon "NewEnumerator2")))

(event Input|EnhancedActionEvents|EnhancedInputActionSecondary_Weapon
  (params (ActionValue :type Boolean) (ElapsedSeconds :type Float%20%28double-precision%29) (TriggeredSeconds :type Float%20%28double-precision%29) (InputAction :type Input%20Action%20Object%20Reference :default "/Game/Blueprints/Player/Inputs/Secondary_Weapon.Secondary_Weapon"))
  ;[1 1 1] Switching Weapon
  (if (Utilities|Enum|NotEqual(Enum) (Variables|Default|GetEquippedWeapon) "NewEnumerator1")
    (CallFunction|SRVEquipWeapon "NewEnumerator1")))

(event Input|EnhancedActionEvents|EnhancedInputActionShoot_Weapon
  (params (ActionValue :type Boolean) (ElapsedSeconds :type Float%20%28double-precision%29) (TriggeredSeconds :type Float%20%28double-precision%29) (InputAction :type Input%20Action%20Object%20Reference :default "/Game/Blueprints/Player/Inputs/Shoot_Weapon.Shoot_Weapon")))

(event EventBeginPlay
  ;[1 1 1] Player Movment
  (bind _playercontroller (Class|INTPlayerController|GetPlayerControllerRef(Message) (Pawn|GetController)))
  (Utilities|IsValid _playercontroller
    (:Is%20Valid
      (Input|AddMappingContext (PlayerController|LocalPlayerSubsystems|GetEnhancedInputLocalPlayerSubsystem _playercontroller) "/Game/Blueprints/Player/Inputs/Default.Default" 0 "(bIgnoreAllPressedKeysUntilRelease=True,bForceImmediately=False,bNotifyUserSettings=False)"))))

(fn ConstructionScript)

(fn FCrouch
  (params (bCrouch :type Boolean))
  (bind _output_get (LocalVariables|SetCrouch%20Local bCrouch))
  (Networking|SwitchHasAuthority
    (:Authority
      _)
    (:Remote
      (CallFunction|SRVCrouch _output_get)))
  (if (LocalVariables|GetCrouch%20Local)
    (Character|Crouch)
    (Variables|Default|SetbCrouch true)
    (else
      (Character|UnCrouch)
      (Variables|Default|SetbCrouch false))))

(fn FWalk
  (params (bWalk :type Boolean))
  (bind _output_get (LocalVariables|SetWalk%20Local bWalk))
  (Networking|SwitchHasAuthority
    (:Authority
      _)
    (:Remote
      (CallFunction|SRVWalk _output_get)))
  (if (LocalVariables|GetWalk%20Local)
    (Variables|/Script/Engine.CharacterMovementComponent|SetMaxWalkSpeed (Variables|Character|GetCharacterMovement) (Variables|Default|GetWalk%20Speed))
    (Variables|Default|SetbWalk true)
    (else
      (Variables|/Script/Engine.CharacterMovementComponent|SetMaxWalkSpeed (Variables|Character|GetCharacterMovement) (Variables|Default|GetRun%20Speed))
      (Variables|Default|SetbWalk false))))

(fn FIsNotJumping
  (return (not (AI|Components|NavMovement|IsFalling (Variables|Character|GetCharacterMovement)))))

(fn FCalculateAimDirection
  (Networking|SwitchHasAuthority
    (:Authority
      _)
    (:Remote
      (CallFunction|SRVCalculateAimDirection)))
  (Variables|Default|SetAimDirection (.Pitch (Math|Rotator|BreakRotator (Math|Rotator|Delta(Rotator) (Pawn|GetControlRotation :!class /Script/Engine.Pawn) (Transformation|GetActorRotation))))))

(fn OnRepLootedWeapon
  (bind _looted_weapon (Variables|Default|GetLooted%20Weapon))
  (bind _weapon (Variables|/Game/Blueprints/Weapons/Weapon_Base.Weapon_Base_C|GetWeapon _looted_weapon))
  (bind _looted_weapon_2 (Variables|Default|GetLooted%20Weapon)
    (:then
      (Physics|SetSimulatePhysics (Variables|/Game/Blueprints/Weapons/Weapon_Base.Weapon_Base_C|GetWeapon _looted_weapon_2) false)
      (Collision|SetCollisionEnabled (Variables|/Game/Blueprints/Weapons/Weapon_Base.Weapon_Base_C|GetWeapon _looted_weapon_2) "NoCollision")
      (Collision|SetCollisionEnabled (Variables|/Game/Blueprints/Weapons/Weapon_Base.Weapon_Base_C|GetCollisionSphere (Variables|Default|GetLooted%20Weapon)) "NoCollision")
      (Transformation|AttachComponentToComponent _weapon (Variables|/Game/Blueprints/Weapons/Weapon_Base.Weapon_Base_C|GetDefaultSceneRoot _looted_weapon) "None" "SnapToTarget" "SnapToTarget" "SnapToTarget" true)
      (Transformation|ResetRelativeTransform _weapon)
      (if (Utilities|Enum|Equal(Enum) (Variables|Default|GetEquippedWeapon) "NewEnumerator0")
        (Transformation|AttachComponentToComponent (Variables|Default|GetLooted%20Weapon) (Variables|Character|GetMesh) (Utilities|Select :Index (.WeaponType (Utilities|Struct|BreakWeapon_Info (CallFunction|FGetWeaponInfo (Variables|/Game/Blueprints/Weapons/Weapon_Base.Weapon_Base_C|GetWeaponName (Variables|Default|GetLooted%20Weapon))))) :NewEnumerator0 "None" :NewEnumerator1 "S_Pistol" :NewEnumerator2 "S_Rifle") "SnapToTarget" "SnapToTarget" "SnapToTarget" true)
        (else
          (Transformation|AttachComponentToComponent (Variables|Default|GetLooted%20Weapon) (Variables|Character|GetMesh) (Utilities|Select :Index (.WeaponType (Utilities|Struct|BreakWeapon_Info (CallFunction|FGetWeaponInfo (Variables|/Game/Blueprints/Weapons/Weapon_Base.Weapon_Base_C|GetWeaponName (Variables|Default|GetLooted%20Weapon))))) :NewEnumerator0 "None" :NewEnumerator1 "S_WeaponSide" :NewEnumerator2 "S_WeaponBack") "SnapToTarget" "SnapToTarget" "SnapToTarget" true))))
    (:else)))

(fn OnRepWeapontoDrop
  (bind _weapontodrop (Variables|Default|GetWeaponToDrop))
  (bind _weapon (Variables|/Game/Blueprints/Weapons/Weapon_Base.Weapon_Base_C|GetWeapon _weapontodrop))
  (bind _weapontodrop_2 (Variables|Default|GetWeaponToDrop)
    (:then
      (Transformation|DetachFromActor _weapontodrop_2 "KeepWorld" "KeepWorld" "KeepWorld")
      (Collision|SetCollisionEnabled _weapon "PhysicsOnly")
      (Physics|SetSimulatePhysics _weapon true)
      (Collision|SetCollisionEnabled (Variables|/Game/Blueprints/Weapons/Weapon_Base.Weapon_Base_C|GetCollisionSphere (Variables|Default|GetWeaponToDrop)) "QueryOnly"))
    (:else)))

(fn FDropWeapon
  (params (WeaponToDrop :type Weapon%20Base%20Object%20Reference))
  (Variables|/Game/Blueprints/Weapons/Weapon_Base.Weapon_Base_C|SetbCanBeInteractedWith WeaponToDrop false)
  (bind _output_get (Variables|Default|SetWeaponToDrop WeaponToDrop))
  (CallFunction|SetDroppedWeapon _output_get)
  (Utilities|Array|RemoveItem (Variables|Default|GetWeaponInventory) WeaponToDrop)
  (if (Utilities|Enum|Equal(Enum) (Variables|Default|GetEquippedWeapon) (.WeaponType (Utilities|Struct|BreakWeapon_Info (CallFunction|FGetWeaponInfo (Variables|/Game/Blueprints/Weapons/Weapon_Base.Weapon_Base_C|GetWeaponName _output_get)))))
    (CallFunction|SetEquippedWeapon "NewEnumerator0")))

(fn OnRepEquipWeapon
  (bind _equipweapon (Variables|Default|GetEquipWeapon)
    (:then
      (Transformation|DetachFromActor _equipweapon "KeepWorld" "KeepWorld" "KeepWorld")
      (Transformation|AttachComponentToComponent (Variables|Default|GetEquipWeapon) (Variables|Character|GetMesh) (Utilities|Select :Index (.WeaponType (Utilities|Struct|BreakWeapon_Info (CallFunction|FGetWeaponInfo (Variables|/Game/Blueprints/Weapons/Weapon_Base.Weapon_Base_C|GetWeaponName (Variables|Default|GetEquipWeapon))))) :NewEnumerator0 "None" :NewEnumerator1 "S_Pistol" :NewEnumerator2 "S_Rifle") "SnapToTarget" "SnapToTarget" "SnapToTarget" true))
    (:else)))

(fn OnRepUnequipWeapon
  (bind _unequipweapon (Variables|Default|GetUnequipWeapon)
    (:then
      (Transformation|DetachFromActor _unequipweapon "KeepWorld" "KeepWorld" "KeepWorld")
      (Transformation|AttachComponentToComponent (Variables|Default|GetUnequipWeapon) (Variables|Character|GetMesh) (Utilities|Select :Index (.WeaponType (Utilities|Struct|BreakWeapon_Info (CallFunction|FGetWeaponInfo (Variables|/Game/Blueprints/Weapons/Weapon_Base.Weapon_Base_C|GetWeaponName (Variables|Default|GetUnequipWeapon))))) :NewEnumerator0 "None" :NewEnumerator1 "S_WeaponSide" :NewEnumerator2 "S_WeaponBack") "SnapToTarget" "SnapToTarget" "SnapToTarget" true))
    (:else)))

(fn GetPlayerBaseRef
  (return self))