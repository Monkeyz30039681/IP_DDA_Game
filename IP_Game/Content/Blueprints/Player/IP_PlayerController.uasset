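; Player controller that manages on-screen widgets, currently the crosshair, and shows it on BeginPlay.
; ShowHideWidget forwards to a CL_ event, likely client-side, which branches to show or hide functions that switch on the widget type.
; The crosshair widget is created lazily on first show, cached, and added to or removed from the viewport.
; GetPlayerControllerRef returns the controller itself.
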(event Custom|ShowHideWidget
  (params (Widget :type Game_UI%20Enum :default "NewEnumerator0") (Show :type Boolean))
  (CallFunction|CLShowHideWidget Widget Show))

(event Custom|CL_ShowHideWidget
  (params (Widget :type Game_UI%20Enum :default "NewEnumerator0") (Show :type Boolean))
  (if Show
    (CallFunction|FShowWidget Widget)
    (else
      (CallFunction|FHideWidget Widget))))

(event EventBeginPlay
  (CallFunction|ShowHideWidget "NewEnumerator0" true))

(fn ConstructionScript)

(fn FShowWidget
  (params (Widget :type Game_UI%20Enum :default "NewEnumerator0"))
  (switch Utilities|FlowControl|Switch|SwitchonGame_UI Widget
    (:NewEnumerator0
      (Variables|Default|GetCrosshair
        (:then
          _)
        (:else
          (bind _returnvalue (UserInterface|CreateWidget "/Game/UI/WB_Crosshair.WB_Crosshair_C"))
          (bind _output_get (Variables|Default|SetCrosshair _returnvalue))))
      (UserInterface|Viewport|AddtoViewport _output_get 0))))

(fn FHideWidget
  (params (Widget :type Game_UI%20Enum :default "NewEnumerator0"))
  (switch Utilities|FlowControl|Switch|SwitchonGame_UI Widget
    (:NewEnumerator0
      (bind _crosshair (Variables|Default|GetCrosshair)
        (:then
          (Widget|RemovefromParent _crosshair))
        (:else)))))

(fn GetPlayerControllerRef
  (return self))